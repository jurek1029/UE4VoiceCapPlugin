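; Test actor that exercises a voice recorder component by capturing a short clip and playing it back.
; On BeginPlay it initializes and starts recording, prints a message if either step fails, then stops after a fixed delay.
; The component's OnCaptureFinished event plays the captured SoundWave as 2D audio, while an alternative play call is left unconnected.
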(event `self.ReceiveBeginPlay`
  (bind _returnvalue (`VoiceRecorderBPLibrary.VoiceRecordedInitFunction` (`self.VoiceRecorder`)))
  (if _returnvalue
    (bind _returnvalue_2 (`VoiceRecorderBPLibrary.VoiceRecordedStartFunction`))
    (if _returnvalue_2
      (`KismetSystemLibrary.Delay` 4.0)
      (`VoiceRecorderBPLibrary.VoiceRecordedStopFunction`)
      (else
        (`KismetSystemLibrary.PrintString` "Voice recorder start fail" true true (struct :`R` 1.0 :`G` 0.008445 :`B` 0.322536 :`A` 1.0))))
    (else
      (`KismetSystemLibrary.PrintString` "Voice recorder init fail" true true (struct :`R` 1.0 :`B` 0.381948 :`A` 1.0)))))

(event `self.VoiceRecorder.OnCaptureFinished`
  (params (soundWave :type "SoundWaveProcedural Object Reference"))
  (`GameplayStatics.PlaySound2D` soundWave 1.0 1.0 0.0 null null))

(fn `UserConstructionScript`)