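; BP_SpawnVoiceRecorder is an actor that plays back audio captured by its VoiceRecorder component.
; BeginPlay initializes the recorder, setting a FirstRun flag on success or printing an error on failure.
; Each finished capture spawns its SoundWave as a 2D sound.
; When a capture starts, it toggles that sound component's active state, skipping this on the first run when no playback exists yet.
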(event `self.ReceiveBeginPlay`
  (bind _returnvalue (`VoiceRecorderBPLibrary.VoiceRecordedInitFunction` (`self.VoiceRecorder`)))
  (if _returnvalue
    (set `self.firstRun` true)
    (else
      (`KismetSystemLibrary.PrintString` "Voice Recorder no initialized From BP_SpawnVoiceREcorder"))))

(event `self.VoiceRecorder.OnCaptureStart`
  (if (`self.firstRun`)
    (set `self.firstRun` false)
    (else
      (`ActorComponent.ToggleActive` (stale `self.VoiceRecorder.OnCaptureFinished` _returnvalue)))))

(event `self.VoiceRecorder.OnCaptureFinished`
  (params (soundWave :type "SoundWaveProcedural Object Reference"))
  (bind _returnvalue (`GameplayStatics.SpawnSound2D` soundWave 1.0 1.0 0.0 null)))

(fn `UserConstructionScript`)